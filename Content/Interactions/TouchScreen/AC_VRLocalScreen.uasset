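; VR actor component that shows a UI widget on a floating touch screen that follows the local player's head.
; Show events async-load the widget class, optionally pass it an init payload, and place it on a BP_TouchScreen child actor, created on first use and then reused.
; While shown, tick keeps the pivot at the camera, smoothly follows head yaw only, and turns the screen toward the viewer.
; Hiding stops tick and visibility after a delay.
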(event `OR_HideScreen`
  (params (AfterSeconds :type "Float (single-precision)"))
  (`KismetSystemLibrary.Delay` AfterSeconds)
  (`self.SetComponentTickEnabled` false)
  (bind _scene (`self.Scene`)
    (:`then`
      (`SceneComponent.SetVisibility` _scene false true))
    (:`else`)))

(event `self.ReceiveBeginPlay`
  (`/Engine/EditorBlueprintResources/StandardMacros.IsValid` (`self.WidgetToDisplay`) ; un petit check parce que parfois le ShowScreen peut être applé avant le begin play
    (:`Is Not Valid`
      (`self.SetComponentTickEnabled` false))))

(event `OR_ShowScreen`
  (params (WidgetToDisplay :type "UserWidget Soft Class Reference") (`Display Size` :type "Vector2D Structure" :default (1280.0 720.0)))
  (bind _class (`|LoadAssetClass` WidgetToDisplay)
    (:`Completed`
      (bind _asuser_widget (castclass `UserWidget` _class))
      (bind _returnvalue (`|CreateWidget` _asuser_widget))
      (`self.ShowScreen` `Display Size` _returnvalue))))

(event `ShowScreenWithPayload`
  (params (WidgetToDisplay :type "UserWidget Soft Class Reference") (`Display Size` :type "Vector2D Structure" :default (1280.0 720.0)) (Payload :type "/VRInteraction/Interactions/TouchScreen/BP_VRScreenGenericPayload Object Reference"))
  (bind _class (`|LoadAssetClass` WidgetToDisplay)
    (:`Completed`
      (bind _asuser_widget (castclass `UserWidget` _class))
      (bind _returnvalue (`|CreateWidget` _asuser_widget))
      (`self.ShowScreen` `Display Size` _returnvalue)
      (message `/VRInteraction/Interactions/TouchScreen/BPI_LocalScreen.HandleInitializationPayload` _returnvalue Payload))))

(event `self.ReceiveTick`
  (params (DeltaSeconds :type "Float (single-precision)"))
  (`parent.ReceiveTick` DeltaSeconds)
  (`self.PerformTick`))

(fn `PerformTick`
  (locals (Camera :type "ReplicatedVRCameraComponent Object Reference") (PlayerHeadRotation :type "Rotator Structure" :default (struct)))
  (bind (_returnvalue_roll _returnvalue_pitch _returnvalue_yaw) (`KismetMathLibrary.BreakRotator` (`SceneComponent.K2_GetComponentRotation` (`local.Camera`))))
  (`/Engine/EditorBlueprintResources/StandardMacros.IsValid` (`self.GetOwner`)
    (:`Is Valid`
      (bind _output_get (set `local.Camera` (`Actor.GetComponentByClass` (`self.GetOwner`) "/Script/VRExpansionPlugin.ReplicatedVRCameraComponent")))
      (`/Engine/EditorBlueprintResources/StandardMacros.IsValid` _output_get
        (:`Is Valid`
          (set `local.PlayerHeadRotation` (`KismetMathLibrary.MakeRotator` 0.0 0.0 _returnvalue_yaw))
          (`SceneComponent.K2_SetWorldRotation` (`self.Scene`) (`KismetMathLibrary.RInterpTo` (`SceneComponent.K2_GetComponentRotation` (`self.Scene`)) (`local.PlayerHeadRotation`) (`GameplayStatics.GetWorldDeltaSeconds`) (`self.Interp Speed`)) false false)
          (`SceneComponent.K2_SetWorldRotation` (`self.Widget`) (`KismetMathLibrary.FindLookAtRotation` (`SceneComponent.K2_GetComponentLocation` (`self.Widget`)) (`SceneComponent.K2_GetComponentLocation` (`local.Camera`))) false false)
          (`SceneComponent.K2_SetWorldLocation` (`self.Scene`) (`SceneComponent.K2_GetComponentLocation` (`local.Camera`)) false false))))))

(fn `ShowScreen`
  (params (`Display Size` :type "Vector2D Structure" :default (1280.0 720.0)) (WidgetToDisplay :type "UserWidget Object Reference"))
  (bind _widget (`self.Widget`))
  (`self.SetComponentTickEnabled` true)
  (set `self.Display Size` `Display Size`)
  (set `self.WidgetToDisplay` WidgetToDisplay)
  (bind _scene (`self.Scene`)
    (:`then`
      (`SceneComponent.SetVisibility` _scene true true)
      (bind _asbp_touch_screen (cast `/VRInteraction/Interactions/TouchScreen/BP_TouchScreen` (`ChildActorComponent.ChildActor` (`self.Widget`))))
      (bind _widgetcomponent (`TouchScreen.WidgetComponent` _asbp_touch_screen))
      (`WidgetComponent.SetWidget` _widgetcomponent (`local.WidgetToDisplay`))
      (`WidgetComponent.SetDrawSize` _widgetcomponent (`self.Display Size`)))
    (:`else`
      (bind _returnvalue (`|AddComponentByClass` (`self.GetOwner`) "/Script/Engine.SceneComponent" true (`KismetMathLibrary.MakeTransform` (0.0 0.0 0.0))))
      (set `self.Scene` _returnvalue)
      (bind _returnvalue_2 (`|AddComponentByClass` (`self.GetOwner`) "/Script/Engine.ChildActorComponent" true (`KismetMathLibrary.MakeTransform` (`self.WidgetOffset`) (struct) (`self.WidgetScale`))))
      (set `self.Widget` _returnvalue_2)
      (`ChildActorComponent.SetChildActorClass` _widget (`self.SurfaceClass`))
      (bind _asbp_touch_screen_2 (cast `/VRInteraction/Interactions/TouchScreen/BP_TouchScreen` (`ChildActorComponent.ChildActor` _widget)))
      (bind _widgetcomponent_2 (`TouchScreen.WidgetComponent` _asbp_touch_screen_2))
      (`WidgetComponent.SetWidget` _widgetcomponent_2 (`local.WidgetToDisplay`))
      (`SceneComponent.K2_AttachToComponent` (`self.Widget`) (`self.Scene`) "None" "KeepRelative" "KeepWorld" "KeepWorld" true)
      (`WidgetComponent.SetDrawSize` _widgetcomponent_2 (`self.Display Size`)))))