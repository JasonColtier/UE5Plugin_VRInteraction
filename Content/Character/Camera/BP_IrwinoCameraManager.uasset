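; Player camera manager that fades the local player's view as if opening or closing the eyes, opening them on BeginPlay.
; A helper finds the locally controlled pawn's mesh tagged "FadeSphere" and caches a dynamic M_ScreenFade material on it.
; A timeline drives that material's opacity, reversing to close and hiding the sphere once fully open.
; Black, Clear and CustomFader events set timeline time from the fading curve's range.
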(event `self.ReceiveBeginPlay`
  ;[1 1 1] au début on voit ce qu'il se passe (écran qui dit patientez)
  (`self.GetFadeSphereMaterialInPawn`
    (:`then`
      (`self.OpenEyes` false))))

(event `OpenEyes`
  (params (FadeAudio :type Boolean))
  (set `self.FadeAudio` FadeAudio)
  ;[0.03434 0.03434 0.03434] goes from 0 to 1
  ;
  ; Play from start 0->1 | value 1->0
  ; Play from end 1->0 | value 0->1
  (bind (_direction _fadetrack) (`Timeline|Timeline` :`NewTime` (`self.ManualTime`) :!label _label)
    (:`Update`
      (bind _mat (`self.GetFadeSphereMaterialInPawn`)
        (:`then`
          (`MaterialInstanceDynamic.SetScalarParameterValue` _mat "Opacity" (- 1.0 _fadetrack)))))
    (:`Finished`
      (`/Engine/EditorBlueprintResources/StandardMacros.IsValid` (`self.FadeSphere`)
        (:`Is Valid`
          (switch `ETimelineDirection` _direction
            (:`Forward`
              (`SceneComponent.SetVisibility` (`self.FadeSphere`) false false))))))))

(event `CloseEyes`
  (params (FadeAudio :type Boolean))
  (bind _fadesphere (`self.FadeSphere`))
  (set `self.FadeAudio` FadeAudio)
  (`/Engine/EditorBlueprintResources/StandardMacros.IsValid` _fadesphere
    (:`Is Valid`
      (`SceneComponent.SetVisibility` _fadesphere true false)
      (goto _label :!via `Reverse`))
    (:`Is Not Valid`
      (goto _label :!via `Reverse`))))

(event `Black`
  (params (FadeAudio :type Boolean))
  ;[1 1 1] removed : caused issues of black screen
  (`self.GetFadeSphereMaterialInPawn`
    (:`then`
      (set `self.FadeAudio` FadeAudio)
      (set `self.ManualTime` (`CurveBase.GetTimeRange` (`self.FadingCurve`)))
      (`SceneComponent.SetVisibility` (`self.FadeSphere`) true false))))

(event `Clear`
  (params (FadeAudio :type Boolean))
  ;[1 1 1] removed : caused issues of black screen
  (set `self.FadeAudio` FadeAudio)
  (set `self.ManualTime` (`.MaxTime` (`CurveBase.GetTimeRange` (`self.FadingCurve`))))
  (`SceneComponent.SetVisibility` (`self.FadeSphere`) false false))

(event `CustomFader`
  (params (FadeValue :type "Float (double-precision)") (FadeAudio :type Boolean))
  (bind (_mintime _maxtime) (`CurveBase.GetTimeRange` (`self.FadingCurve`)))
  ;[1 1 1] removed : caused issues of black screen
  (set `self.FadeAudio` FadeAudio)
  (set `self.ManualTime` (`KismetMathLibrary.MapRangeClamped` FadeValue 0.0 1.0 _mintime _maxtime)))

(fn `UserConstructionScript`)